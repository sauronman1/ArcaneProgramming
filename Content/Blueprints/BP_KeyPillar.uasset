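; BP_KeyPillar is a pillar that lowers a referenced Door when a BP_KeyPlate physics body is near it.
; Each Tick it runs a sphere overlap at its location and adds delta time to a Timer while a plate is found.
; Until that cumulative, never-reset Timer passes six seconds, it draws a debug sphere and offsets the Door downward by a fixed, frame-rate-dependent step without sweeping.
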(event `self.ReceiveTick`
  (params (DeltaSeconds :type "Float (single-precision)"))
  (bind _returnvalue (`self.K2_GetActorLocation`))
  (bind (_outactors _returnvalue_2) (`KismetSystemLibrary.SphereOverlapActors` _returnvalue 120.0 (`|MakeArray` "ObjectTypeQuery4" :!type "EObjectTypeQuery Enum") "/Game/Blueprints/BP_KeyPlate.BP_KeyPlate_C"))
  (if _returnvalue_2
    (bind _output_get (set `self.Timer` (+ (`self.Timer`) (`GameplayStatics.GetWorldDeltaSeconds`))))
    (if (<= _output_get 6.0)
      (`KismetSystemLibrary.DrawDebugSphere` _returnvalue 120.0)
      (`self.K2_AddActorWorldOffset` (`self.Door`) (0.0 0.0 -2.0) false false))))

(fn `UserConstructionScript`)